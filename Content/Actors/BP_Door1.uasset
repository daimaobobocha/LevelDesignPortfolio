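; BP_Door1 is a door actor that the player opens with the E key while overlapping it.
; Overlap by a BP_ShooterCharacter enables the actor's input for player 0, so E hides the Cube and turns off its collision.
; Leaving the overlap restores the Cube's visibility and collision and disables input again, closing the door without animation.
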(event `Key|E`
  (params (Key :type "Key Structure"))
  (bind _cube (`self.Cube`))
  (:`Pressed`
    (`SceneComponent.SetVisibility` _cube false false)
    (`PrimitiveComponent.SetCollisionEnabled` _cube "NoCollision")))

(event `self.ReceiveActorEndOverlap`
  (params (OtherActor :type "Actor Object Reference"))
  (bind _cube (`self.Cube`))
  (cast `/Game/Variant_Shooter/Blueprints/BP_ShooterCharacter` OtherActor)
  (`SceneComponent.SetVisibility` _cube true false)
  (`PrimitiveComponent.SetCollisionEnabled` _cube "QueryAndPhysics")
  (`self.DisableInput` (`GameplayStatics.GetPlayerController` 0)))

(event `self.ReceiveActorBeginOverlap`
  (params (OtherActor :type "Actor Object Reference"))
  (cast `/Game/Variant_Shooter/Blueprints/BP_ShooterCharacter` OtherActor)
  (`self.EnableInput` (`GameplayStatics.GetPlayerController` 0)))

(fn `UserConstructionScript`)