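; Door actor that opens on the E key once it has been unlocked by a matching key index.
; An Unlock event compares the incoming index with DoorIndex, sets Unlocked and hides Cube2.
; Overlap with BP_ShooterCharacter enables or disables input from player controller 0.
; Opening hides Cube and Cube1 and removes collision from Cube, with no animation or closing logic.
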(event `Unlock`
  (params (KeyIndex :type Integer))
  (if (== KeyIndex (`self.DoorIndex`))
    (set `self.Unlocked?` true)
    (`SceneComponent.SetVisibility` (`self.Cube2`) false false)))

(event `self.ReceiveActorBeginOverlap`
  (params (OtherActor :type "Actor Object Reference"))
  (cast `/Game/Variant_Shooter/Blueprints/BP_ShooterCharacter` OtherActor)
  (`self.EnableInput` (`GameplayStatics.GetPlayerController` 0)))

(event `self.ReceiveActorEndOverlap`
  (params (OtherActor :type "Actor Object Reference"))
  (cast `/Game/Variant_Shooter/Blueprints/BP_ShooterCharacter` OtherActor)
  (`self.DisableInput` (`GameplayStatics.GetPlayerController` 0)))

(event `Key|E` :consume false
  (params (Key :type "Key Structure"))
  (:`Pressed`
    (if (`self.Unlocked?`)
      (`SceneComponent.SetVisibility` (`self.Cube1`) false false)
      (`SceneComponent.SetVisibility` (`self.Cube`) false false)
      (`PrimitiveComponent.SetCollisionEnabled` (`self.Cube`) "NoCollision"))))

(fn `UserConstructionScript`)