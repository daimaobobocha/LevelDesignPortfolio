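; BP_Door_OneSide is a one-sided door that the player must first reach from the far side before it can be opened.
; Overlapping Colide4 permanently sets Othersideopened, swaps the Cube3/Cube1 visuals and enables input; later actor overlaps enable input only when that flag is set.
; Pressing E opens it instantly by hiding meshes, disabling Cube collision and playing audio.
; Ending overlap restores it, disables input and plays a second sound if opened.
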(event `self.ReceiveBeginPlay`
  (`SceneComponent.SetVisibility` (`self.Cube1`) false false))

(event `Key|E`
  (params (Key :type "Key Structure"))
  (:`Pressed`
    (`SceneComponent.SetVisibility` (`self.Cube`) false false)
    (`SceneComponent.SetVisibility` (`self.Cube1`) false false)
    (`SceneComponent.SetVisibility` (`self.Cube2`) false false)
    (`PrimitiveComponent.SetCollisionEnabled` (`self.Cube`) "NoCollision")
    (`AudioComponent.Play` (`self.Audio`) 0.0)
    (set `self.oppened?` true)))

(event `self.ReceiveActorEndOverlap`
  (params (OtherActor :type "Actor Object Reference"))
  (cast `/Game/Variant_Shooter/Blueprints/BP_ShooterCharacter` OtherActor)
  (`SceneComponent.SetVisibility` (`self.Cube`) true false)
  (`SceneComponent.SetVisibility` (`self.Cube1`) true false)
  (`SceneComponent.SetVisibility` (`self.Cube2`) true false)
  (`PrimitiveComponent.SetCollisionEnabled` (`self.Cube`) "QueryAndPhysics")
  (`self.DisableInput` null)
  (if (`self.oppened?`)
    (`AudioComponent.Play` (`self.Audio1`) 0.0)
    (set `self.oppened?` false)))

(event `self.ReceiveActorBeginOverlap`
  (params (OtherActor :type "Actor Object Reference"))
  (cast `/Game/Variant_Shooter/Blueprints/BP_ShooterCharacter` OtherActor)
  (if (`self.othersideopened?`)
    (`self.EnableInput` (`GameplayStatics.GetPlayerController` 0))))

(event `self.colide4.OnComponentBeginOverlap`
  (params (OverlappedComponent :type "PrimitiveComponent Object Reference") (OtherActor :type "Actor Object Reference") (OtherComp :type "PrimitiveComponent Object Reference") (OtherBodyIndex :type Integer) (bFromSweep :type Boolean) (SweepResult :type "HitResult Structure (by ref)"))
  (cast `/Game/Variant_Shooter/Blueprints/BP_ShooterCharacter` OtherActor)
  (set `self.othersideopened?` true)
  (`self.EnableInput` (`GameplayStatics.GetPlayerController` 0))
  (`SceneComponent.SetVisibility` (`self.Cube1`) true false)
  (`SceneComponent.SetVisibility` (`self.Cube3`) false false))

(fn `UserConstructionScript`)