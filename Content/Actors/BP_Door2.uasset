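; BP_Door2 is a proximity door that BP_ShooterCharacter opens with the E key.
; Overlap events enable and disable the actor's input for player 0, so E works only nearby.
; Opening hides three cube meshes, disables the main cube's collision and plays a sound; leaving restores both.
; The Opened flag is never reset, so after a first opening every exit plays the second sound.
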(event `Key|E`
  (params (Key :type "Key Structure"))
  (:`Pressed`
    (`SceneComponent.SetVisibility` (`self.Cube1`) false false)
    (`SceneComponent.SetVisibility` (`self.Cube`) false false)
    (`SceneComponent.SetVisibility` (`self.Cube2`) false false)
    (`PrimitiveComponent.SetCollisionEnabled` (`self.Cube`) "NoCollision")
    (`AudioComponent.Play` (`self.Audio`) 0.8)
    (set `self.Opened?` true)))

(event `self.ReceiveActorEndOverlap`
  (params (OtherActor :type "Actor Object Reference"))
  (cast `/Game/Variant_Shooter/Blueprints/BP_ShooterCharacter` OtherActor)
  (`SceneComponent.SetVisibility` (`self.Cube1`) true false)
  (`SceneComponent.SetVisibility` (`self.Cube`) true false)
  (`SceneComponent.SetVisibility` (`self.Cube2`) true false)
  (`PrimitiveComponent.SetCollisionEnabled` (`self.Cube`) "QueryAndPhysics")
  (`self.DisableInput` (`GameplayStatics.GetPlayerController` 0))
  (if (`self.Opened?`)
    (`AudioComponent.Play` (`self.Audio1`) 0.0)
    (set `self.Opened?` true)))

(event `self.ReceiveActorBeginOverlap`
  (params (OtherActor :type "Actor Object Reference"))
  (cast `/Game/Variant_Shooter/Blueprints/BP_ShooterCharacter` OtherActor)
  (`self.EnableInput` (`GameplayStatics.GetPlayerController` 0)))

(fn `UserConstructionScript`)